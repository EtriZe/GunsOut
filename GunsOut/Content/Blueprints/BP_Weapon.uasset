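; BP_Weapon is a weapon actor with a Paper2D sprite that destroys itself when overlapped, after printing the other actor's name.
; On BeginPlay, InitValues reads the hardcoded "Glock" row of DT_Weapons into ammo, damage, fire rate and bullet speed variables and sets the sprite skin.
; A random row pick is present but unused, and the overlap passes no stats to the other actor.
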(event `self.ReceiveBeginPlay`
  (`self.InitValues`))

(event `self.PaperSprite.OnComponentBeginOverlap`
  (params (OverlappedComponent :type "PrimitiveComponent Object Reference") (OtherActor :type "Actor Object Reference") (OtherComp :type "PrimitiveComponent Object Reference") (OtherBodyIndex :type Integer) (bFromSweep :type Boolean) (SweepResult :type "HitResult Structure (by ref)"))
  (`KismetSystemLibrary.PrintString` (`KismetSystemLibrary.GetDisplayName` OtherActor))
  (`self.K2_DestroyActor` self))

(fn `InitValues`
  (bind _outrownames (`DataTableFunctionLibrary.GetDataTableRowNames` "/Game/Blueprints/DT_Weapons.DT_Weapons"))
  (bind _returnvalue (`|GetDataTableRow` "/Game/Blueprints/DT_Weapons.DT_Weapons" "Glock")
    (:`then`
      (set `self.Munitions` (break `/Game/Blueprints/ST_Weapons` _returnvalue))
      (set `self.Dégats` (`.Dégats_8_1E15D07047F0B83F718AF1B0415BD9A3` (break `/Game/Blueprints/ST_Weapons` _returnvalue)))
      (set `self.Cadence` (`.Cadence_5_D24002DF43A91239933054A1F510E451` (break `/Game/Blueprints/ST_Weapons` _returnvalue)))
      (set `self.VitesseBalles` (`.VitesseBalles_9_B5AF2948484140240C075A9AB9F1448A` (break `/Game/Blueprints/ST_Weapons` _returnvalue)))
      (`PaperSpriteComponent.SetSprite` (`self.PaperSprite`) (`.Skin_13_9265921349154A639C73A6B4C09FCBE6` (break `/Game/Blueprints/ST_Weapons` _returnvalue))))
    (:`RowNotFound`
      (`KismetSystemLibrary.PrintString` "Gun non trouvé dans Data Table"))))

(fn `UserConstructionScript`)