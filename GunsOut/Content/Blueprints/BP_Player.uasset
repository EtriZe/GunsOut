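; Player character for a 2D flipbook platformer, driven by Enhanced Input using the P1 mapping context added on BeginPlay.
; Move input drives movement along world X and flips control yaw to face the direction of travel.
; Jump input starts and stops the built-in Character jump through a wrapper; both jump and movement wrappers are marked temporary.
; Each tick selects the idle, run, rise or fall flipbook from ground state and velocity.
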(event `self.ReceiveBeginPlay`
  (bind _asplayer_controller (cast `PlayerController` (`self.GetController`)))
  (`EnhancedInputSubsystemInterface.AddMappingContext` (pcsubsystem `EnhancedInputLocalPlayerSubsystem` _asplayer_controller) "/Game/Input/IMC_PlatformingP1.IMC_PlatformingP1" 0 (struct)))

(event `EnhancedInput|/Game/Input/Actions/IA_JumpP1`
  (params (ActionValue :type Boolean) (ElapsedSeconds :type "Float (double-precision)") (TriggeredSeconds :type "Float (double-precision)") (InputAction :type "InputAction Object Reference" :default "/Game/Input/Actions/IA_JumpP1.IA_JumpP1"))
  (:`Triggered`
    (`self.CustomJump` true))
  (:`Completed`
    (`self.CustomJump` false)))

(event `self.ReceiveTick`
  (params (DeltaSeconds :type "Float (single-precision)"))
  (`self.UpdateAnimation`))

(event `EnhancedInput|/Game/Input/Actions/IA_MoveP1`
  (params (ActionValue :type "Float (double-precision)") (ElapsedSeconds :type "Float (double-precision)") (TriggeredSeconds :type "Float (double-precision)") (InputAction :type "InputAction Object Reference" :default "/Game/Input/Actions/IA_MoveP1.IA_MoveP1"))
  (:`Triggered`
    (`self.CustomMovement` ActionValue)))

(fn `CustomJump`
  (params (Jump :type Boolean))
  (if Jump
    ;[1 1 1] Temp
    (`self.Jump`)
    (else
      (`self.StopJumping`))))

(fn `CustomMovement`
  (params (`Scale Value` :type "Float (double-precision)"))
  ;[1 1 1] Temp
  (`self.AddMovementInput` (1.0 0.0 0.0) `Scale Value`) ; Movement on X axis
  (`Controller.SetControlRotation` (`self.GetController`) (select `bool` (> `Scale Value` 0.0) :`false` (`KismetMathLibrary.MakeRotator` 0.0 0.0 180.0) :`true` (`KismetMathLibrary.MakeRotator` 0.0))))

(fn `UpdateAnimation`
  (bind (_returnvalue_x _returnvalue_y _returnvalue_z) (`KismetMathLibrary.BreakVector` (`self.GetVelocity`)))
  (if (`NavMovementComponent.IsMovingOnGround` (`self.CharacterMovement`))
    (if (> (`KismetMathLibrary.VSize` (`self.GetVelocity`)) 0.0)
      (`PaperFlipbookComponent.SetFlipbook` (`self.Sprite`) "/Game/PaperAssets/Character/FlipBooks/Player_Run.Player_Run")
      (else
        (`PaperFlipbookComponent.SetFlipbook` (`self.Sprite`) "/Game/PaperAssets/Character/FlipBooks/Player_Idle.Player_Idle")))
    (elif (< _returnvalue_z -100.0)
      (`PaperFlipbookComponent.SetFlipbook` (`self.Sprite`) "/Game/PaperAssets/Character/FlipBooks/Player_Fall.Player_Fall")
      (else
        (`PaperFlipbookComponent.SetFlipbook` (`self.Sprite`) "/Game/PaperAssets/Character/FlipBooks/Player_JumpRise.Player_JumpRise")))))

(fn `UserConstructionScript`)