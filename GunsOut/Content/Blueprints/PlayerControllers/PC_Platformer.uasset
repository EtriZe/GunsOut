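; Player controller for networked platformer play that spawns each player's BP_Player and sets up camera and input.
; BeginPlay runs a client-to-server RPC chain that spawns the pawn at the first unused Spawn actor, marks it used, and possesses it.
; On possess, the view switches to the first StageCamera and a client RPC adds the IMC_PlatformingP1 Enhanced Input mapping context.
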(event `self.ReceiveBeginPlay`
  (`self.Client_SpawnPlayer`))

(event `Client_SpawnPlayer`
  (`self.Server_SpawnPlayer`))

(event `Server_SpawnPlayer`
  (bind _returnvalue (`self.SpawnPlayer`))
  (`self.Possess` _returnvalue))

(event `self.ReceivePossess`
  (params (PossessedPawn :type "Pawn Object Reference"))
  (bind _outactors (`GameplayStatics.GetAllActorsOfClass` "/Game/Blueprints/StageCamera.StageCamera_C"))
  (`self.SetViewTargetWithBlend` (`|GetArrayItem` _outactors))
  (`self.Client_SetInput`))

(event `Client_SetInput`
  (`EnhancedInputSubsystemInterface.AddMappingContext` (pcsubsystem `EnhancedInputLocalPlayerSubsystem` (`GameplayStatics.GetPlayerController` 0)) "/Game/Input/IMC_PlatformingP1.IMC_PlatformingP1" 0 (struct)))

(fn `GetSpawnLocation`
  (returns (SpawnTransform :type "Transform Structure (by ref)"))
  (bind _outactors (`GameplayStatics.GetAllActorsOfClass` "/Game/Blueprints/Spawn.Spawn_C"))
  (for _array_element _outactors
    (if (not (`/Game/Blueprints/Spawn.Used` _array_element))
      (set `/Game/Blueprints/Spawn.Used` true _array_element)
      (return (`self.GetTransform` _array_element)))))

(fn `SpawnPlayer`
  (returns (ReturnValue :type "/Game/Blueprints/BP_Player Object Reference"))
  (bind _spawntransform (`self.GetSpawnLocation`))
  (bind _returnvalue (`|SpawnActorFromClass` "/Game/Blueprints/BP_Player.BP_Player_C" _spawntransform "Undefined" "MultiplyWithRoot" null null))
  (return _returnvalue))

(fn `UserConstructionScript`)